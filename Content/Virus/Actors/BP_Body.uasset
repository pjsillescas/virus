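; BP_Body is an actor for the Virus card game that holds one organ slot per color: red, green, blue, yellow and multicolor.
; AddOrgan spawns a BP_Organ from a card at that color's arrow component, returning false if the slot is already filled.
; GetOrganOfColor looks up a slot, and IsComplete checks whether enough organs have a qualifying status to meet a given threshold.
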(event EventBeginPlay)

(event Collision|EventActorBeginOverlap
  (params (OtherActor :type Actor%20Object%20Reference)))

(event EventTick
  (params (DeltaSeconds :type Float%20%28single-precision%29)))

(fn ConstructionScript)

(fn AddOrgan
  (params (Card :type BP%20Card%20Object%20Reference))
  (switch Utilities|FlowControl|Switch|SwitchonE_CardColor (.color (Variables|/Game/Virus/SinglePlayer/BP_Card.BP_Card_C|GetData Card))
    (:NewEnumerator0
      (Utilities|IsValid (Variables|Default|GetRedOrgan)
        (:Is%20Valid
          (return false))
        (:Is%20Not%20Valid
          (bind _organ (CallFunction|SpawnOrgan (Variables|Default|GetRedArrow) Card))
          (Variables|Default|SetRedOrgan _organ)
          (return true))))
    (:NewEnumerator1
      (Utilities|IsValid (Variables|Default|GetGreenOrgan)
        (:Is%20Valid
          (return false))
        (:Is%20Not%20Valid
          (bind _organ_2 (CallFunction|SpawnOrgan (Variables|Default|GetGreenArrow) Card))
          (Variables|Default|SetGreenOrgan _organ_2)
          (return true))))
    (:NewEnumerator2
      (Utilities|IsValid (Variables|Default|GetBlueOrgan)
        (:Is%20Valid
          (return false))
        (:Is%20Not%20Valid
          (bind _organ_3 (CallFunction|SpawnOrgan (Variables|Default|GetBlueArrow) Card))
          (Variables|Default|SetBlueOrgan _organ_3)
          (return true))))
    (:NewEnumerator3
      (Utilities|IsValid (Variables|Default|GetYellowOrgan)
        (:Is%20Valid
          (return false))
        (:Is%20Not%20Valid
          (bind _organ_4 (CallFunction|SpawnOrgan (Variables|Default|GetYellowArrow) Card))
          (Variables|Default|SetYellowOrgan _organ_4)
          (return true))))
    (:NewEnumerator4
      (Utilities|IsValid (Variables|Default|GetMulticolorOrgan)
        (:Is%20Valid
          (return false))
        (:Is%20Not%20Valid
          (bind _organ_5 (CallFunction|SpawnOrgan (Variables|Default|GetMulticolorArrow) Card))
          (Variables|Default|SetMulticolorOrgan _organ_5)
          (return true))))))

(fn SpawnOrgan
  (params (Spawn%20Transform%20Location :type Arrow%20Component%20Object%20Reference) (Card :type BP%20Card%20Object%20Reference))
  (bind _returnvalue (Game|SpawnActorfromClass "/Game/Virus/Actors/BP_Organ.BP_Organ_C" (Math|Transform|MakeTransform (Transformation|GetWorldLocation Spawn%20Transform%20Location) "0, 0, 0" "1,1,1") "AlwaysSpawn" 0 Card 0))
  (return _returnvalue))

(fn IsComplete
  (params (Threshold :type Integer))
  (for _array_element (Utilities|Array|MakeArray (Variables|Default|GetGreenOrgan) (Variables|Default|GetBlueOrgan) (Variables|Default|GetRedOrgan) (Variables|Default|GetYellowOrgan) (Variables|Default|GetMulticolorOrgan))
    (Utilities|IsValid _array_element
      (:Is%20Valid
        (if (Math|Boolean|ORBoolean (Utilities|Enum|Equal(Enum) (Variables|/Game/Virus/Actors/BP_Organ.BP_Organ_C|GetStatus _array_element) "NewEnumerator0") (Utilities|Enum|Equal(Enum) (Variables|/Game/Virus/Actors/BP_Organ.BP_Organ_C|GetStatus _array_element) "NewEnumerator2") (Utilities|Enum|Equal(Enum) (Variables|/Game/Virus/Actors/BP_Organ.BP_Organ_C|GetStatus _array_element) "NewEnumerator3"))
          (Math|Integer|IncrementInt (LocalVariables|GetLCount))))))
  (return (>= (LocalVariables|GetLCount) Threshold)))

(fn GetOrganOfColor
  (params (Color :type E_CardColor%20Enum :default "NewEnumerator0"))
  (Utilities|FlowControl|Sequence
    (:then_0
      (switch Utilities|FlowControl|Switch|SwitchonE_CardColor Color
        (:NewEnumerator0
          (LocalVariables|SetLOrgan (Variables|Default|GetRedOrgan)))
        (:NewEnumerator1
          (LocalVariables|SetLOrgan (Variables|Default|GetGreenOrgan)))
        (:NewEnumerator2
          (LocalVariables|SetLOrgan (Variables|Default|GetBlueOrgan)))
        (:NewEnumerator3
          (LocalVariables|SetLOrgan (Variables|Default|GetYellowOrgan)))
        (:NewEnumerator4
          (LocalVariables|SetLOrgan (Variables|Default|GetMulticolorOrgan)))))
    (:then_1
      (return (LocalVariables|GetLOrgan)))))