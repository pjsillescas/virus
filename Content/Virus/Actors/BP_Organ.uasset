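; BP_Organ is the board actor for an organ card in the Virus card game, colored from its card data and showing a status widget while selected.
; Selection swaps its mesh to a glow material.
; ApplyCard accepts same-color or multicolor medicine and virus cards, driving a Healthy, Infected, Vaccinated and Inmune state machine.
; Opposing cards cancel out, a second virus destroys the organ, and spent cards are discarded through BP_SinglePlayerController.
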(event EventBeginPlay
  (bind _aswbp_organ_status (Utilities|Casting|CastToWBP_OrganStatus (UserInterface|GetWidget (Variables|Default|GetWidgetStatus))))
  (Variables|/Game/Virus/UI/WBP_OrganStatus.WBP_OrganStatus_C|SetOrgan _aswbp_organ_status self)
  (Rendering|SetVisibility (Variables|Default|GetWidgetStatus) false false)
  (Variables|Default|SetColor (.color (Variables|/Game/Virus/SinglePlayer/BP_Card.BP_Card_C|GetData (Variables|Default|GetCard))))
  (CallFunction|SetColor))

(event Collision|EventActorBeginOverlap
  (params (OtherActor :type Actor%20Object%20Reference)))

(event EventTick
  (params (DeltaSeconds :type Float%20%28single-precision%29)))

(fn ConstructionScript
  (CallFunction|SetColor))

(fn SetColor
  (Utilities|FlowControl|Sequence
    (:then_0
      (switch Utilities|FlowControl|Switch|SwitchonE_CardColor (Variables|Default|GetColor)
        (:NewEnumerator0
          (LocalVariables|SetLMaterial "/Game/Virus/Materials/MI_Red.MI_Red"))
        (:NewEnumerator1
          (LocalVariables|SetLMaterial "/Game/Virus/Materials/MI_Green.MI_Green"))
        (:NewEnumerator2
          (LocalVariables|SetLMaterial "/Game/Virus/Materials/MI_Blue.MI_Blue"))
        (:NewEnumerator3
          (LocalVariables|SetLMaterial "/Game/Virus/Materials/MI_Yellow.MI_Yellow"))
        (:NewEnumerator4
          (LocalVariables|SetLMaterial "/Game/Virus/Materials/MI_Multicolor.MI_Multicolor"))))
    (:then_1
      (Rendering|Material|SetMaterial (Variables|Default|GetStaticMesh) 0 (LocalVariables|GetLMaterial)))))

(fn Select
  (CallFunction|SetSelectedColor)
  (Rendering|SetVisibility (Variables|Default|GetWidgetStatus) true false))

(fn Deselect
  (CallFunction|SetColor)
  (Rendering|SetVisibility (Variables|Default|GetWidgetStatus) false false))

(fn SetSelectedColor
  (Utilities|FlowControl|Sequence
    (:then_0
      (switch Utilities|FlowControl|Switch|SwitchonE_CardColor (Variables|Default|GetColor)
        (:NewEnumerator0
          (LocalVariables|SetLMaterial "/Game/Virus/Materials/MI_GlowRed.MI_GlowRed"))
        (:NewEnumerator1
          (LocalVariables|SetLMaterial "/Game/Virus/Materials/MI_GlowGreen.MI_GlowGreen"))
        (:NewEnumerator2
          (LocalVariables|SetLMaterial "/Game/Virus/Materials/MI_GlowBlue.MI_GlowBlue"))
        (:NewEnumerator3
          (LocalVariables|SetLMaterial "/Game/Virus/Materials/MI_GlowYellow.MI_GlowYellow"))
        (:NewEnumerator4
          (LocalVariables|SetLMaterial "/Game/Virus/Materials/MI_GlowMulticolor.MI_GlowMulticolor"))))
    (:then_1
      (Rendering|Material|SetMaterial (Variables|Default|GetStaticMesh) 0 (LocalVariables|GetLMaterial)))))

(fn ApplyCard
  (params (Card :type BP%20Card%20Object%20Reference))
  (bind _data (Variables|/Game/Virus/SinglePlayer/BP_Card.BP_Card_C|GetData Card))
  (bind (_name _description _type _color) (Utilities|Struct|BreakS_Card _data))
  (if (or (Utilities|Enum|Equal(Enum) (Variables|Default|GetColor) _color) (Utilities|Enum|Equal(Enum) _color "NewEnumerator4"))
    (switch Utilities|FlowControl|Switch|SwitchonE_CardType _type
      (:NewEnumerator1
        (CallFunction|ApplyMedicine Card))
      (:NewEnumerator2
        (CallFunction|ApplyVirus Card)))))

(fn ApplyMedicine
  (params (Card :type BP%20Card%20Object%20Reference))
  (switch Utilities|FlowControl|Switch|SwitchonE_OrganStatus (Variables|Default|GetStatus)
    (:NewEnumerator0
      (Variables|Default|SetStatus "NewEnumerator2")
      (Utilities|Array|Add (Variables|Default|GetMedicines) 0 :!label _label))
    (:NewEnumerator1
      (Variables|Default|SetStatus "NewEnumerator0")
      (CallFunction|DiscardCard Card)
      (CallFunction|DiscardCard (Utilities|Array|Get(acopy) (Variables|Default|GetViruses)))
      (Utilities|Array|RemoveIndex (Variables|Default|GetViruses)))
    (:NewEnumerator2
      (Variables|Default|SetStatus "NewEnumerator3")
      (goto _label))))

(fn ApplyVirus
  (params (Card :type BP%20Card%20Object%20Reference%20%28by%20ref%29))
  (switch Utilities|FlowControl|Switch|SwitchonE_OrganStatus (Variables|Default|GetStatus)
    (:NewEnumerator0
      (Variables|Default|SetStatus "NewEnumerator1")
      (Utilities|Array|Add (Variables|Default|GetViruses) Card))
    (:NewEnumerator1
      (Utilities|Array|Add (Variables|Default|GetViruses) Card)
      (CallFunction|DestroyOrgan))
    (:NewEnumerator2
      (Variables|Default|SetStatus "NewEnumerator0")
      (CallFunction|DiscardCard Card)
      (CallFunction|DiscardCard (Utilities|Array|Get(acopy) (Variables|Default|GetMedicines)))
      (Utilities|Array|RemoveIndex (Variables|Default|GetMedicines)))))

(fn DestroyOrgan
  (for _array_element (Variables|Default|GetMedicines)
    (CallFunction|DiscardCard _array_element))
  (for _array_element_2 (Variables|Default|GetViruses)
    (CallFunction|DiscardCard _array_element_2))
  (CallFunction|DiscardCard (Variables|Default|GetCard))
  (Actor|DestroyActor))

(fn DiscardCard
  (params (Card :type BP%20Card%20Object%20Reference))
  (bind _asbp_single_player_controller (Utilities|Casting|CastToBP_SinglePlayerController (Game|GetPlayerController 0)))
  (Default|DiscardCard _asbp_single_player_controller Card))