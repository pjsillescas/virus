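; Player controller for the single-player Virus card game, bridging the HUD, mouse input and the player pawn.
; On BeginPlay it creates the HUD in Game and UI mode, hands it to the pawn and blends the view to the first CameraActor.
; Card play, discard and end-turn events forward to the pawn, with end turn refilling the hand.
; Left click traces under the cursor to set or clear the pawn's selected organ.
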(event Custom|PlayCard
  (params (Data :type S%20Card%20Structure) (Index :type Integer))
  (Default|PlayCard (Variables|Default|GetPlayerPawn) Data Index))

(event Custom|EndTurn
  (Default|FillHand (Variables|Default|GetPlayerPawn)))

(event Custom|DiscardCard
  (params (Index :type Integer))
  (Default|DiscardCard (Variables|Default|GetPlayerPawn) Index))

(event EventBeginPlay
  (CallFunction|SetupWidgets)
  (bind _asbp_single_player_pawn (Utilities|Casting|CastToBP_SinglePlayerPawn (Game|Player|GetPlayerPawn 0)))
  (bind _output_get (Variables|Default|SetPlayerPawn _asbp_single_player_pawn))
  (Default|SetupWidgets _output_get (Variables|Default|GetHud))
  (bind _outactors (Actor|GetAllActorsOfClass "/Script/Engine.CameraActor"))
  (Game|Player|SetViewTargetwithBlend (Utilities|Array|Get(acopy) _outactors) 1.0 "VTBlend_Linear" 0.0 false))

(event EventTick
  (params (DeltaSeconds :type Float%20%28single-precision%29)))

(event Input|MouseEvents|LeftMouseButton
  (params (Key :type Key%20Structure :default "None"))
  (bind (_worldlocation _worlddirection) (Game|Player|ConvertMouseLocationToWorldSpace))
  (:Pressed
    (bind _outhit (Collision|LineTraceForObjects _worldlocation (+ _worldlocation (* _worlddirection (Variables|Default|GetTraceLength))) (Utilities|Array|MakeArray "ObjectTypeQuery2") false 0 "None"))
    (bind _asbp_organ (Utilities|Casting|CastToBP_Organ (.HitActor (Collision|BreakHitResult _outhit)))
      (:then
        (Default|SetSelectedOrgan (Variables|Default|GetPlayerPawn) _asbp_organ))
      (:CastFailed
        (Default|SetSelectedOrgan (Variables|Default|GetPlayerPawn))))))

(fn ConstructionScript)

(fn SetupWidgets
  (bind _returnvalue (UserInterface|CreateWidget "/Game/Virus/UI/WBP_SinglePlayerHud.WBP_SinglePlayerHud_C" self))
  (bind _output_get (Variables|Default|SetHud _returnvalue))
  (Variables|Default|SetHandWidget (Variables|/Game/Virus/UI/WBP_SinglePlayerHud.WBP_SinglePlayerHud_C|GetWBP_Hand _output_get))
  (UserInterface|Viewport|AddtoViewport (Variables|Default|GetHud) 0)
  (Input|SetInputModeGameandUI self (Variables|Default|GetHud) "DoNotLock" false)
  (Variables|Default|SetbShowMouseCursor true))