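; Base pawn for the single-player Virus card game, holding a player's hand, body and selected organ.
; It refills its hand through BP_SinglePlayerGameMode and mirrors it in the HUD's hand widget.
; PlayCard routes by card type: organs join the body, while medicines and viruses apply to the selected organ after a color and status check, with HUD notifications on failure.
; The five treatment card handlers are empty stubs.
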(event Custom|PlayCard
  (params (Card :type BP%20Card%20Object%20Reference))
  (switch Utilities|FlowControl|Switch|SwitchonE_CardType (.Type (Utilities|Struct|BreakS_Card (Variables|/Game/Virus/SinglePlayer/BP_Card.BP_Card_C|GetData Card)))
    (:NewEnumerator0
      (CallFunction|PlayOrgan Card))
    (:NewEnumerator1
      (CallFunction|PlayMedicine Card))
    (:NewEnumerator2
      (CallFunction|PlayVirus Card))
    (:NewEnumerator3
      (CallFunction|PlayTransplant Card))
    (:NewEnumerator4
      (CallFunction|PlayContagion Card))
    (:NewEnumerator5
      (CallFunction|PlayOrganThief Card))
    (:NewEnumerator6
      (CallFunction|PlayLatexGlove Card))
    (:NewEnumerator7
      (CallFunction|PlayMedicalError Card))))

(event Custom|DiscardCard
  (params (Card :type BP%20Card%20Object%20Reference))
  (Default|Discard (Variables|Default|GetGameMode) Card)
  (CallFunction|DiscardfromHand Card))

(event Custom|PlayLatexGlove
  (params (Card :type BP%20Card%20Object%20Reference)))

(event Custom|PlayMedicalError
  (params (Card :type BP%20Card%20Object%20Reference)))

(event Custom|DiscardFromHand
  (params (Card :type BP%20Card%20Object%20Reference%20%28by%20ref%29))
  (Utilities|Array|RemoveItem (Variables|Default|GetHand) Card)
  (CallFunction|DisplayHand)
  (Utilities|IsValid (Variables|Default|GetHandWidget)
    (:Is%20Valid
      (Default|SetSelectedCard (Variables|Default|GetHandWidget))
      (Development|PrintString "Discard from hand"))))

(event Custom|SetupWidgets
  (params (Hud :type WBP%20Single%20Player%20Hud%20Object%20Reference))
  (bind _output_get (Variables|Default|SetHud Hud))
  (Variables|Default|SetHandWidget (Variables|/Game/Virus/UI/WBP_SinglePlayerHud.WBP_SinglePlayerHud_C|GetWBP_HandPlayer _output_get))
  (CallFunction|FillHand))

(event Custom|SetSelectedOrgan
  (params (SelectedOrgan :type BP%20Organ%20Object%20Reference))
  (Utilities|IsValid (Variables|Default|GetSelectedOrgan)
    (:Is%20Valid
      (Default|Deselect (Variables|Default|GetSelectedOrgan)))
    (:Is%20Not%20Valid
      _))
  (bind _output_get (Variables|Default|SetSelectedOrgan SelectedOrgan))
  (Utilities|IsValid _output_get
    (:Is%20Valid
      (Default|Select (Variables|Default|GetSelectedOrgan)))))

(event Custom|FillHand
  (Utilities|IsValid (Variables|Default|GetGameMode)
    (:Is%20Valid
      (bind _filledhand (Default|FillHand (Variables|Default|GetGameMode) (Variables|Default|GetHand)))
      (Variables|Default|SetHand _filledhand)
      (CallFunction|DisplayHand))))

(event Custom|DisplayHand
  (Utilities|IsValid (Variables|Default|GetHandWidget)
    (:Is%20Valid
      (Default|Clear (Variables|Default|GetHandWidget))
      (for _array_element (Variables|Default|GetHand)
        (Default|AddCard (Variables|Default|GetHandWidget) _array_element)))))

(event Custom|PlayOrgan
  (params (Card :type BP%20Card%20Object%20Reference))
  (bind _bsuccess (Default|AddOrgan (Variables|Default|GetBody) Card))
  (if _bsuccess
    (CallFunction|DiscardfromHand Card)
    (else
      (Default|ShowNotification (Variables|Default|GetHud) (Utilities|Text|FormatText "{color} organ already exists" (Utilities|String|EnumtoString (.Color (Utilities|Struct|BreakS_Card (Variables|/Game/Virus/SinglePlayer/BP_Card.BP_Card_C|GetData Card)))))))))

(event Custom|PlayMedicine
  (params (Card :type BP%20Card%20Object%20Reference))
  (if (CallFunction|IsCompatiblewithSelectedOrgan Card)
    (Default|ApplyCard (Variables|Default|GetSelectedOrgan) Card)
    (CallFunction|DiscardfromHand Card)
    (else
      (Default|ShowNotification (Variables|Default|GetHud) (Utilities|Text|MakeLiteralText "Invalid organ")))))

(event Custom|PlayVirus
  (params (Card :type BP%20Card%20Object%20Reference))
  (if (CallFunction|IsCompatiblewithSelectedOrgan Card)
    (Default|ApplyCard (Variables|Default|GetSelectedOrgan) Card)
    (CallFunction|DiscardfromHand Card)
    (else
      (Default|ShowNotification (Variables|Default|GetHud) (Utilities|Text|MakeLiteralText "Invalid organ")))))

(event Custom|PlayTransplant
  (params (Card :type BP%20Card%20Object%20Reference)))

(event Custom|PlayContagion
  (params (Card :type BP%20Card%20Object%20Reference)))

(event Custom|PlayOrganThief
  (params (Card :type BP%20Card%20Object%20Reference)))

(event EventBeginPlay
  (bind _asbp_single_player_game_mode (Utilities|Casting|CastToBP_SinglePlayerGameMode (Game|GetGameMode)))
  (Variables|Default|SetGameMode _asbp_single_player_game_mode)
  (CallFunction|FillHand))

(event Collision|EventActorBeginOverlap
  (params (OtherActor :type Actor%20Object%20Reference)))

(event EventTick
  (params (DeltaSeconds :type Float%20%28single-precision%29)))

(fn ConstructionScript)

(fn IsCompatiblewithSelectedOrgan
  (params (Card :type BP%20Card%20Object%20Reference%20%28by%20ref%29))
  (bind _selectedorgan (Variables|Default|GetSelectedOrgan))
  (bind _data (Variables|/Game/Virus/SinglePlayer/BP_Card.BP_Card_C|GetData Card))
  (bind _color (Utilities|Struct|BreakS_Card _data))
  (bind _color_2 (Variables|/Game/Virus/Actors/BP_Organ.BP_Organ_C|GetColor _selectedorgan))
  (Utilities|IsValid _selectedorgan
    (:Is%20Valid
      (return (and (Math|Boolean|ORBoolean (Utilities|Enum|Equal(Enum) _color_2 _color) (Utilities|Enum|Equal(Enum) _color_2 "NewEnumerator4") (Utilities|Enum|Equal(Enum) _color "NewEnumerator4")) (Utilities|Enum|NotEqual(Enum) (Variables|/Game/Virus/Actors/BP_Organ.BP_Organ_C|GetStatus _selectedorgan) "NewEnumerator3"))))
    (:Is%20Not%20Valid
      (return false))))