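; Single-player game mode for a card game in which the player and adversaries each build a body, won by completing it with enough healthy organs.
; On BeginPlay it creates draw and discard decks, then identifies the player's body by object name and hands it to the pawn.
; Hand refills merge the discard pile back when the deck runs short.
; Ending a turn checks every body, then either triggers the controller's game over or rotates the turn.
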(event EventBeginPlay
  (bind _returnvalue (Game|ConstructObjectfromClass "/Game/Virus/SinglePlayer/BP_Deck.BP_Deck_C" self))
  (bind _output_get (Variables|Default|SetDeck _returnvalue))
  (Default|CreateDeck _output_get)
  (bind _returnvalue_2 (Game|ConstructObjectfromClass "/Game/Virus/SinglePlayer/BP_Deck.BP_Deck_C" self))
  (Variables|Default|SetDiscardDeck _returnvalue_2)
  (bind _outactors (Actor|GetAllActorsOfClass "/Game/Virus/Actors/BP_Body.BP_Body_C"))
  (for _array_element _outactors
    (if (Utilities|Enum|Equal(Enum) (Utilities|GetObjectName _array_element) "PlayerBody")
      (Variables|Default|SetPlayerBody _array_element)
      (bind _asbp_single_player_pawn (Utilities|Casting|CastToBP_SinglePlayerPawn (Game|Player|GetPlayerPawn 0)))
      (Variables|/Game/Virus/SinglePlayer/BP_BaseSinglePlayerPawn.BP_BaseSinglePlayerPawn_C|SetBody _asbp_single_player_pawn (Variables|Default|GetPlayerBody))
      (else
        (Utilities|Array|Add (Variables|Default|GetAdversaryBodies) _array_element)))))

(event EventTick
  (params (DeltaSeconds :type Float%20%28single-precision%29)))

(fn ConstructionScript)

(fn FillHand
  (params (Hand :type Array%20of%20BP%20Card%20Object%20References))
  (bind _returnvalue (Utilities|Array|Length Hand))
  (bind _maxcardsinhand (Variables|Default|GetMaxCardsInHand))
  (bind _maxcardsinhand_2 (Variables|Default|GetMaxCardsInHand))
  (bind _returnvalue_2 (- _maxcardsinhand _returnvalue))
  (bind _returnvalue_3 (Math|Integer|Clamp(Integer) _returnvalue_2 0 _maxcardsinhand_2))
  (if (> _returnvalue_3 0)
    (if (< (Default|GetCardCount (Variables|Default|GetDeck)) _returnvalue_3)
      (Default|Merge (Variables|Default|GetDeck) (Variables|Default|GetDiscardDeck))
      (Default|EmptyDeck (Variables|Default|GetDiscardDeck)))
    (bind _drawncards (Default|Draw (Variables|Default|GetDeck) _returnvalue_3))
    (for _array_element _drawncards
      (Utilities|Array|Add Hand _array_element)))
  (return Hand))

(fn Discard
  (params (Card :type BP%20Card%20Object%20Reference))
  (Default|AddCard (Variables|Default|GetDiscardDeck) Card)
  (Development|PrintString "discard"))

(fn CheckforFinishedGame
  (if (Default|IsComplete (Variables|Default|GetPlayerBody) (Variables|Default|GetHealthyOrgansThreshold))
    (bind _asbp_single_player_controller (Utilities|Casting|CastToBP_SinglePlayerController (Game|GetPlayerController 0)))
    (Default|GameOver _asbp_single_player_controller)
    (return true)
    (else
      (for _array_element (Variables|Default|GetAdversaryBodies)
        (if (Default|IsComplete _array_element (Variables|Default|GetHealthyOrgansThreshold))
          (bind _asbp_single_player_controller_2 (Utilities|Casting|CastToBP_SinglePlayerController (Game|GetPlayerController 0)))
          (Default|GameOver _asbp_single_player_controller_2 (Utilities|String|Replace (Utilities|GetObjectName _array_element) "Body"))
          (return true)))
      (return false))))

(fn EndTurn
  (bind _bgameisfinished (CallFunction|CheckforFinishedGame))
  (if (not _bgameisfinished)
    (Variables|Default|SetPlayerTurn (Math|Integer|%(Integer) (+ (Variables|Default|GetPlayerTurn) 1) (+ (Utilities|Array|Length (Variables|Default|GetAdversaryBodies)) 1)))))