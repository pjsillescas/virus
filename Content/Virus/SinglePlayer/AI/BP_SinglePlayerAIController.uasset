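; AI controller for the single-player adversary in the turn-based Virus game.
; It lazily sets up the adversary blackboard, stores its own turn id there and starts the adversary behavior tree, then mirrors the current player turn into the blackboard.
; Ending a turn refills the controlled pawn's hand and hands control back to the single-player game mode.
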(event Custom|EndTurn
  (Default|FillHand (Variables|Default|GetControlledPawn))
  (Default|EndTurn (Variables|Default|GetGameMode)))

(event Custom|SetTurnId
  (params (TurnId :type Integer))
  (Class|BlackboardComponent|SetValueasInt (CallFunction|GetBlackboardComponent) (Utilities|Name|MakeLiteralName "MyTurnId") TurnId)
  (AI|RunBehaviorTree "/Game/Virus/SinglePlayer/AI/BT_SinglePlayerAdversary.BT_SinglePlayerAdversary"))

(event Custom|SetCurrentPlayerTurn
  (params (PlayerTurn :type Integer))
  (Class|BlackboardComponent|SetValueasInt (CallFunction|GetBlackboardComponent) (Utilities|Name|MakeLiteralName "PlayerTurn") PlayerTurn))

(event EventBeginPlay
  (bind _asbp_single_player_game_mode (Utilities|Casting|CastToBP_SinglePlayerGameMode (Game|GetGameMode)))
  (Variables|Default|SetGameMode _asbp_single_player_game_mode)
  (bind _asbp_single_player_adversary_pawn (Utilities|Casting|CastToBP_SinglePlayerAdversaryPawn (Pawn|GetControlledPawn)))
  (Variables|Default|SetControlledPawn _asbp_single_player_adversary_pawn))

(event EventTick
  (params (DeltaSeconds :type Float%20%28single-precision%29)))

(fn ConstructionScript)

(fn GetBlackboardComponent
  (Utilities|IsValid (Variables|Default|GetBoackboard)
    (:Is%20Valid
      _)
    (:Is%20Not%20Valid
      (bind _blackboardcomponent (Class|AIController|UseBlackboard "/Game/Virus/SinglePlayer/AI/BB_SinglePlayerAdversary.BB_SinglePlayerAdversary"))
      (Variables|Default|SetBoackboard _blackboardcomponent)))
  (return (Variables|Default|GetBoackboard)))