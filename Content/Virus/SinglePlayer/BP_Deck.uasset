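; BP_Deck is the card deck for the single-player Virus game, holding the pool of BP_Card objects.
; CreateDeck reads every DT_Deck row, constructs as many cards as its Number field specifies, then shuffles them.
; Draw repeatedly calls DrawSingleCard, which removes a card at a random index rather than from the top.
; Helpers add a card, empty or count the deck, and merge another deck into this one, emptying the source.
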(fn CreateDeck
  (bind _outrownames (DataTable|GetDataTableRowNames "/Game/Virus/Data/DT_Deck.DT_Deck"))
  (for _array_element _outrownames
    (bind _returnvalue (Utilities|GetDataTableRow "/Game/Virus/Data/DT_Deck.DT_Deck" _array_element)
      (:then
        (for _index (range 1 (.Number (Utilities|Struct|BreakS_Card _returnvalue)))
          (bind _returnvalue_2 (Game|ConstructObjectfromClass "/Game/Virus/SinglePlayer/BP_Card.BP_Card_C" self _returnvalue))
          (Utilities|Array|Add (Variables|Default|GetCards) _returnvalue_2)))))
  (CallFunction|Shuffle))

(fn Shuffle
  (Utilities|Array|Shuffle (Variables|Default|GetCards)))

(fn Draw
  (params (NumCards :type Integer))
  (for _index (range 1 NumCards)
    (bind _card (CallFunction|DrawSingleCard))
    (Utilities|Array|Add (LocalVariables|GetLCards) _card))
  (return (LocalVariables|GetLCards)))

(fn DrawSingleCard
  (LocalVariables|SetLIndex (Math|Random|RandomIntegerinRange 0 (- (Utilities|Array|Length (Variables|Default|GetCards)) 1)))
  (LocalVariables|SetLCard (Utilities|Array|Get(acopy) (Variables|Default|GetCards) (LocalVariables|GetLIndex)))
  (Utilities|Array|RemoveIndex (Variables|Default|GetCards) (LocalVariables|GetLIndex))
  (return (LocalVariables|GetLCard)))

(fn EmptyDeck
  (Utilities|Array|Clear (Variables|Default|GetCards)))

(fn AddCard
  (params (Card :type BP%20Card%20Object%20Reference))
  (Utilities|Array|Add (Variables|Default|GetCards) Card))

(fn Merge
  (params (AnotherDeck :type BP%20Deck%20Object%20Reference))
  (for _array_element (Variables|BP_Deck_C|GetCards AnotherDeck)
    (Utilities|Array|Add (Variables|Default|GetCards) _array_element))
  (CallFunction|EmptyDeck AnotherDeck))

(fn GetCardCount
  (return (Utilities|Array|Length (Variables|Default|GetCards))))